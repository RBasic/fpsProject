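; BP_Target is a shootable target actor that awards points to the player when a projectile hits it.
; Its Construction Script applies a StaticMesh variable to the Test component.
; When a FirstPersonProjectile hits that component, it adds ValTarget to the score on player zero's FirstPersonCharacter, then destroys both the projectile and itself.
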(event `self.Test.OnComponentHit`
  (params (HitComponent :type "PrimitiveComponent Object Reference") (OtherActor :type "Actor Object Reference") (OtherComp :type "PrimitiveComponent Object Reference") (NormalImpulse :type "Vector Structure") (Hit :type "HitResult Structure (by ref)"))
  (bind _asfirst_person_projectile (cast `/Game/FirstPersonBP/Blueprints/FirstPersonProjectile` OtherActor))
  (bind _asfirst_person_character (cast `/Game/FirstPersonBP/Blueprints/FirstPersonCharacter` (`GameplayStatics.GetPlayerCharacter` 0)))
  (`/Game/FirstPersonBP/Blueprints/FirstPersonCharacter.IncrementScore` _asfirst_person_character (`self.ValTarget`))
  (`self.K2_DestroyActor` _asfirst_person_projectile)
  (`self.K2_DestroyActor`))

(fn `UserConstructionScript`
  (`StaticMeshComponent.SetStaticMesh` (`self.Test`) (`self.StaticMesh`)))